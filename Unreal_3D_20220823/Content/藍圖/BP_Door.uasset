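; BP_Door is a door that opens only when the player has collected enough bottles.
; When a BP_Player overlaps its Box trigger, the collected bottle count is compared with the player's maximum.
; If it is met, the 開爽 timeline drives the door mesh's relative Z location to open it.
; Otherwise a message is printed saying more bottles are needed.
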(event `self.Box.OnComponentBeginOverlap`
  (params (OverlappedComponent :type "PrimitiveComponent Object Reference") (OtherActor :type "Actor Object Reference") (OtherComp :type "PrimitiveComponent Object Reference") (OtherBodyIndex :type Integer) (bFromSweep :type Boolean) (SweepResult :type "HitResult Structure (by ref)"))
  (bind _asbp_player (cast `/Game/藍圖/BP_Player` OtherActor))
  (if (>= (`/Game/藍圖/BP_Player.取得瓶子數量` _asbp_player) (`/Game/藍圖/BP_Player.最大瓶子數量` _asbp_player))
    (bind (_direction `_開門爽爽`) (`Timeline|開爽`)
      (:`Update`
        (`SceneComponent.K2_SetRelativeLocation` (`self.Door`) (`KismetMathLibrary.MakeVector` 0.0 0.0 `_開門爽爽`) false false)))
    (else
      (`KismetSystemLibrary.PrintString` "瓶子不夠你爽,需要更多瓶子"))))

(fn `UserConstructionScript`)