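; BP_EndLight is an end trigger actor with a box volume and four point lights.
; When BP_Player overlaps the box and the mouse cursor is hidden, it adds the BP_End widget to the viewport and shows the cursor.
; It then plays a timeline that animates the relative locations of the four lights.
; The cursor visibility doubles as a guard against retriggering while the end screen is up.
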(event `self.Box.OnComponentBeginOverlap`
  (params (OverlappedComponent :type "PrimitiveComponent Object Reference") (OtherActor :type "Actor Object Reference") (OtherComp :type "PrimitiveComponent Object Reference") (OtherBodyIndex :type Integer) (bFromSweep :type Boolean) (SweepResult :type "HitResult Structure (by ref)"))
  (bind _returnvalue (`GameplayStatics.GetPlayerController` 0))
  (cast `/Game/藍圖/BP_Player` OtherActor)
  (if (not (`PlayerController.bShowMouseCursor` _returnvalue))
    (bind _returnvalue_2 (`|CreateWidget` "/Game/藍圖/BP_End.BP_End_C"))
    (`UserWidget.AddToViewport` _returnvalue_2 0)
    (set `PlayerController.bShowMouseCursor` true _returnvalue)
    (bind (_direction _light0 _light1 _light2 _light3) (`Timeline|爽到不行`)
      (:`Update`
        (`SceneComponent.K2_SetRelativeLocation` (`self.PointLight`) _light0 false false)
        (`SceneComponent.K2_SetRelativeLocation` (`self.PointLight1`) _light1 false false)
        (`SceneComponent.K2_SetRelativeLocation` (`self.PointLight2`) _light2 false false)
        (`SceneComponent.K2_SetRelativeLocation` (`self.PointLight3`) _light3 false false)))))

(fn `UserConstructionScript`)